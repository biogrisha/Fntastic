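; Turtle actor that, on Activate, travels the length of an assigned SplinePath once and then disappears.
; A slowed WalkingTimeline sets its location and rotation from distance along the spline, using world-space location but local-space rotation.
; A parallel Acceleration timeline ramps the Speed variable up at the start and reverses when the walk ends.
; When that reverse finishes, the turtle spawns smoke, plays a sound and destroys itself.
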(event EventActivate
  (bind _returnvalue (Transformation|GetActorLocation))
  (bind _splinepath (Variables|Default|GetSplinePath))
  (bind _splinecomponent (Variables|/Game/MyContent/Blueprints/SplinePath.SplinePath_C|GetSplineComponent _splinepath))
  (Utilities|IsValid (Variables|Default|GetSplinePath)
    (:Is%20Valid
      (Components|Timeline|SetPlayRate (Variables|Default|GetWalkingTimeline) 0.2)
      (Utilities|FlowControl|Sequence
        (:then_0
          (bind _newtrack_2 (Timeline|WalkingTimeline PlayFromStart)
            (:Update
              (Transformation|SetActorTransform (Math|Transform|MakeTransform (Spline|GetLocationatDistanceAlongSpline _splinecomponent (* (Spline|GetSplineLength _splinecomponent) _newtrack_2) "World") (Spline|GetRotationatDistanceAlongSpline _splinecomponent (* (Spline|GetSplineLength _splinecomponent) _newtrack_2) "Local") "1,1,1")))
            (:Finished
              (bind (_direction _newtrack_0) (Timeline|Acceleration Reverse)
                (:Update
                  (Variables|Default|SetSpeed _newtrack_0))
                (:Finished
                  (if (Utilities|Enum|Equal(Enum) _direction "Backward")
                    (Effects|SpawnEmitteratLocation "/Game/MyContent/Assets/Effects/Smoke.Smoke" _returnvalue "0, 0, 0" "2.000000,2.000000,2.000000")
                    (Audio|PlaySoundatLocation "/Game/MyContent/Assets/Sounds/Spawn_Cue.Spawn_Cue" _returnvalue "0, 0, 0" 1.0 1.0 0.0 0 0 0)
                    (Actor|DestroyActor)))))))
        (:then_1
          (Timeline|Acceleration PlayFromStart))))))

(fn ConstructionScript
  (|CallParentFunction))