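; Blueprint that spawns the WBP_Buttons UI and binds it to three nest references for button-driven interaction.
; On BeginPlay it creates the widget, adds it to the viewport and passes its Nest1, Nest2 and Nest3 variables into the widget's matching variables.
; It then shows the mouse cursor and ignores move input on the first player controller, leaving the player in a point-and-click state.
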(event EventBeginPlay
  (bind _returnvalue (Game|GetPlayerController 0))
  (bind _returnvalue_2 (UserInterface|CreateWidget "/Game/MyContent/Blueprints/WBP_Buttons.WBP_Buttons_C"))
  (bind _output_get (Variables|Default|SetWidget _returnvalue_2))
  (UserInterface|Viewport|AddtoViewport _output_get 0)
  (Variables|/Game/MyContent/Blueprints/WBP_Buttons.WBP_Buttons_C|SetNest1 (Variables|Default|GetWidget) (Variables|Default|GetNest1))
  (Variables|/Game/MyContent/Blueprints/WBP_Buttons.WBP_Buttons_C|SetNest2 (Variables|Default|GetWidget) (Variables|Default|GetNest2))
  (Variables|/Game/MyContent/Blueprints/WBP_Buttons.WBP_Buttons_C|SetNest3 (Variables|Default|GetWidget) (Variables|Default|GetNest3))
  (Variables|/Script/Engine.PlayerController|SetbShowMouseCursor _returnvalue true)
  (Input|SetIgnoreMoveInput _returnvalue true))

(fn ConstructionScript)